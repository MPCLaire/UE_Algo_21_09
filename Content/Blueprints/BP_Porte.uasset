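; BP_Porte is a door that toggles between open and closed when its Activate event is called.
; Activate checks IsOpen and calls OpenDoor or CloseDoor, which set the flag and play or reverse the OpenDoorTL timeline.
; The timeline lerps the Pivot's relative yaw from zero to DoorOpen, but on finish applies that yaw as world rotation.
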(event Custom|OpenDoor
  ;[1 1 1] Ouvrir et fermer la porte
  (Variables|Default|SetIsOpen true)
  (bind _newtrack_0 (Timeline|OpenDoorTL Play)
    (:Update
      (Transformation|SetRelativeRotation (Variables|Default|GetPivot) (Math|Rotator|MakeRotator 0.0 0.0 (Math|Float|Lerp 0.0 (Variables|Default|GetDoorOpen) _newtrack_0)) false false))
    (:Finished
      (Transformation|SetWorldRotation (Variables|Default|GetPivot) (Math|Rotator|MakeRotator 0.0 0.0 (Math|Float|Lerp 0.0 (Variables|Default|GetDoorOpen) _newtrack_0)) false false))))

(event Custom|Close%20Door
  ;[1 1 1] Ouvrir et fermer la porte
  (Variables|Default|SetIsOpen false)
  (bind _newtrack_0 (Timeline|OpenDoorTL Reverse)
    (:Update
      (Transformation|SetRelativeRotation (Variables|Default|GetPivot) (Math|Rotator|MakeRotator 0.0 0.0 (Math|Float|Lerp 0.0 (Variables|Default|GetDoorOpen) _newtrack_0)) false false))
    (:Finished
      (Transformation|SetWorldRotation (Variables|Default|GetPivot) (Math|Rotator|MakeRotator 0.0 0.0 (Math|Float|Lerp 0.0 (Variables|Default|GetDoorOpen) _newtrack_0)) false false))))

(event EventActivate
  (if (Variables|Default|GetIsOpen)
    (CallFunction|CloseDoor)
    (else
      (CallFunction|OpenDoor))))

(fn ConstructionScript)