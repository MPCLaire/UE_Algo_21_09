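; BP_Door3 is a toggleable door that reports its state changes to a referenced lamp, apparently as part of an enigma.
; ToggleDoor3 checks IsOpen, calls OpenDoor or CloseDoor, then notifies LampRef through RemoveDoorsOpen or AddDoorsClosed.
; A timeline lerps the mesh's relative yaw from DoorOpening to zero, reversing from the end to close.
; Its Finished pin applies the same yaw as world rotation, unlike the relative update.
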(event Custom|OpenDoor
  ;[1 1 1] Ouvrir et fermer la porte
  (Variables|Default|SetIsOpen true)
  (bind _newtrack_0 (Timeline|Timeline Play)
    (:Update
      (Transformation|SetRelativeRotation (Variables|Default|GetStaticMesh) (Math|Rotator|MakeRotator 0.0 0.0 (Math|Float|Lerp (Variables|Default|GetDoorOpening) 0.0 _newtrack_0)) false false))
    (:Finished
      (Transformation|SetWorldRotation (Variables|Default|GetStaticMesh) (Math|Rotator|MakeRotator 0.0 0.0 (Math|Float|Lerp (Variables|Default|GetDoorOpening) 0.0 _newtrack_0)) false false))))

(event Custom|Close%20Door
  ;[1 1 1] Ouvrir et fermer la porte
  (Variables|Default|SetIsOpen false)
  (bind _newtrack_0 (Timeline|Timeline ReverseFromEnd)
    (:Update
      (Transformation|SetRelativeRotation (Variables|Default|GetStaticMesh) (Math|Rotator|MakeRotator 0.0 0.0 (Math|Float|Lerp (Variables|Default|GetDoorOpening) 0.0 _newtrack_0)) false false))
    (:Finished
      (Transformation|SetWorldRotation (Variables|Default|GetStaticMesh) (Math|Rotator|MakeRotator 0.0 0.0 (Math|Float|Lerp (Variables|Default|GetDoorOpening) 0.0 _newtrack_0)) false false))))

(fn ConstructionScript)

(fn ToggleDoor3
  (if (Variables|Default|GetIsOpen)
    (CallFunction|CloseDoor)
    (Default|AddDoorsClosed (Variables|Default|GetLampRef))
    (else
      (CallFunction|OpenDoor)
      (Default|RemoveDoorsOpen (Variables|Default|GetLampRef)))))